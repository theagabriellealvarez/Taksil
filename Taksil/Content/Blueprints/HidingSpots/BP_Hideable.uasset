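; Clickable hiding spot that lets the player (BP_Tina) hide when within range, highlighting through custom depth on hover.
; Clicking hides the pawn, shows a widget, fades to the spot's view and activates the QTE.
; Unhide restores player and camera, triggering a caught event if Ernie is in the room.
; Clamped look input feeds a Delay-looped MoveCamera event, which nothing here starts.
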(event `self.ReceiveBeginPlay`
  ;[1 1 1] Initialize
  (bind _returnvalue (`|CreateWidget` "/Game/Blueprints/Widgets/BP_HideInteractable.BP_HideInteractable_C"))
  (set `self.HideWidget` _returnvalue)
  (bind _asbp_tina (cast `/Game/Blueprints/Player/BP_Tina` (`GameplayStatics.GetPlayerPawn` 0)))
  (set `self.As Player` _asbp_tina)
  (bind _asbp_tina_controller (cast `/Game/Blueprints/Player/BP_TinaController` (`GameplayStatics.GetPlayerController` 0)))
  (set `self.playerController` _asbp_tina_controller)
  (bind _asbp_game_mode (cast `/Game/Blueprints/GameMode/BP_GameMode` (`GameplayStatics.GetGameMode`)))
  (set `self.As BP Game Mode` _asbp_game_mode))

(event `CheckDistance`
  ;[1 1 1] Check Distance
  (if (not (`/Game/Blueprints/Player/BP_Tina.isInteracting` (`self.As Player`)))
    (bind _output_get (set `self.isWithinDistance` (< (`KismetMathLibrary.Vector_Distance` (`self.K2_GetActorLocation` self) (`self.K2_GetActorLocation` (`self.As Player`))) 300.0)))
    (if _output_get
      _)))

(event `self.ReceiveActorBeginCursorOver`
  (if (`/Game/Blueprints/GameMode/BP_GameMode.isPlayerHiding` (`self.As BP Game Mode`))
    _
    (elif (not (`/Game/Blueprints/Player/BP_Tina.isInteracting` (`self.As Player`)))
      (set `PlayerController.CurrentMouseCursor` "GrabHandClosed" (`self.playerController`))
      (`PrimitiveComponent.SetRenderCustomDepth` (`self.StaticMesh`) true))))

(event `self.ReceiveActorEndCursorOver`
  (set `PlayerController.CurrentMouseCursor` "Default" (`self.playerController`))
  (`PrimitiveComponent.SetRenderCustomDepth` (`self.StaticMesh`) false))

(event `self.ReceiveActorOnClicked`
  (params (ButtonPressed :type "Key Structure"))
  (bind _returnvalue (`GameplayStatics.GetPlayerCameraManager` 0))
  (bind _as_player (`self.As Player`))
  (bind _durationswitchcamera (`self.DurationSwitchCamera`))
  (bind _as_bp_game_mode (`self.As BP Game Mode`))
  ;[1 1 1] Hide Player
  (if (`/Game/Blueprints/GameMode/BP_GameMode.isPlayerCaught` _as_bp_game_mode)
    _
    (elif (not (`/Game/Blueprints/GameMode/BP_GameMode.isPlayerHiding` _as_bp_game_mode))
      (`self.CheckDistance`)
      (if (`self.isWithinDistance`)
        (set `/Game/Blueprints/Player/BP_Tina.CurrentHidable` self (`self.As Player`))
        (set `/Game/Blueprints/GameMode/BP_GameMode.isPlayerHiding` true (`self.As BP Game Mode`))
        (`UserWidget.AddToViewport` (`self.HideWidget`) 0)
        (`self.SetActorHiddenInGame` _as_player true)
        (`self.SetActorEnableCollision` _as_player false)
        (`self.DisableInput` (`self.playerController`) null)
        (`self.EnableInput` (`GameplayStatics.GetPlayerController` 0))
        (`PlayerCameraManager.StartCameraFade` :`self` _returnvalue :`ToAlpha` 1.0 :`Duration` (`self.DurationSwitchCamera`) :`bHoldWhenFinished` true)
        (`KismetSystemLibrary.Delay` _durationswitchcamera)
        (`PlayerCameraManager.StartCameraFade` :`self` _returnvalue :`FromAlpha` 1.0 :`Duration` _durationswitchcamera :`bHoldWhenFinished` true)
        (`/Game/Blueprints/Player/BP_TinaController.MoveCameraTo` (`/Game/Blueprints/Player/BP_Tina.As Player Controller` (`self.As Player`)) self 0.0)
        (bind _returnvalue_2 (`GameplayStatics.GetActorOfClass` "/Game/Blueprints/Interactables/BP_QTE_Interactable.BP_QTE_Interactable_C"))
        (`/Game/Blueprints/Interactables/BP_QTE_Interactable.ActivateQTE` _returnvalue_2)
        (set `PlayerController.CurrentMouseCursor` "Default" (`self.playerController`))))))

(event `Unhide`
  (bind _returnvalue (`GameplayStatics.GetPlayerCameraManager` 0))
  (bind _as_bp_game_mode (`self.As BP Game Mode`))
  (bind _as_player (`self.As Player`))
  (bind _as_player_2 (`self.As Player`))
  (bind _durationswitchcamera (`self.DurationSwitchCamera`))
  ;[1 1 1] Unhide Player
  (set `/Game/Blueprints/GameMode/BP_GameMode.isPlayerHiding` false (`self.As BP Game Mode`))
  (`PlayerCameraManager.StartCameraFade` :`self` _returnvalue :`ToAlpha` 1.0 :`Duration` (`self.DurationSwitchCamera`) :`bHoldWhenFinished` true)
  (`KismetSystemLibrary.Delay` _durationswitchcamera)
  (`PlayerCameraManager.StartCameraFade` :`self` _returnvalue :`FromAlpha` 1.0 :`Duration` _durationswitchcamera :`bHoldWhenFinished` true)
  (set `/Game/Blueprints/Player/BP_Tina.CurrentHidable` null _as_player_2)
  (`self.SetActorHiddenInGame` _as_player_2 false)
  (`self.SetActorEnableCollision` _as_player_2 true)
  (`self.EnableInput` (`self.playerController`) null)
  (`/Game/Blueprints/Player/BP_TinaController.MoveCameraTo` (`/Game/Blueprints/Player/BP_Tina.As Player Controller` _as_player) (`ActorComponent.GetOwner` (`/Game/Blueprints/Player/BP_Tina.PlayerCamera` _as_player)) 0.0)
  (if (`/Game/Blueprints/GameMode/BP_GameMode.isErnieInRoom` _as_bp_game_mode)
    (set `/Game/Blueprints/GameMode/BP_GameMode.isPlayerCaught` true _as_bp_game_mode)
    (`/Game/Blueprints/GameMode/BP_GameMode.PlayerCaught` _as_bp_game_mode)))

(event `InputAxis|LookUp`
  (params (AxisValue :type "Float (single-precision)"))
  ;[1 1 1] If we want to move the camera :DD nvm might not be possible but yeah
  (if (`/Game/Blueprints/GameMode/BP_GameMode.isPlayerHiding` (`self.As BP Game Mode`))
    (bind _output_get (set `self.Pitch` (`KismetMathLibrary.FClamp` (+ AxisValue (`self.Pitch`)) -40.0 20.0)))))

(event `MoveCamera`
  ;[1 1 1] If we want to move the camera :DD nvm might not be possible but yeah
  (if (`/Game/Blueprints/GameMode/BP_GameMode.isPlayerHiding` (`self.As BP Game Mode`))
    (`SceneComponent.K2_SetRelativeRotation` (`self.Camera`) (`KismetMathLibrary.MakeRotator` 0.0 (stale `InputAxis|LookUp` _output_get) (stale `InputAxis|Turn` _output_get)) false false)
    (`KismetSystemLibrary.Delay` 0.001)
    (`self.MoveCamera`)))

(event `InputAxis|Turn`
  (params (AxisValue :type "Float (single-precision)"))
  ;[1 1 1] If we want to move the camera :DD nvm might not be possible but yeah
  (if (`/Game/Blueprints/GameMode/BP_GameMode.isPlayerHiding` (`self.As BP Game Mode`))
    (bind _output_get (set `self.Yaw` (`KismetMathLibrary.FClamp` (+ (`self.Yaw`) AxisValue) -60.0 60.0)))))

(fn `UserConstructionScript`)