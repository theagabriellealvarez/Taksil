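; BP_CoffeeTable is a clickable interactable that shows dialogue the first time the player clicks it.
; On click it calls the parent handler, then checks and sets a HasInteracted flag so the dialogue fires only once.
; It creates a BP_DialogueOverlay widget, passes in its DialogueToDisplay, and adds it to the viewport.
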(event `self.ReceiveActorOnClicked`
  (params (ButtonPressed :type "Key Structure"))
  (`parent.ReceiveActorOnClicked` "None")
  (if (not (`self.hasInteracted`))
    (set `self.hasInteracted` true)
    (bind _returnvalue (`|GenericCreateObject` "/Game/Blueprints/DialogueSystem/BP_DialogueOverlay.BP_DialogueOverlay_C"))
    (bind _output_get (set `self.DialogueRef` _returnvalue))
    (set `/Game/Blueprints/DialogueSystem/BP_DialogueOverlay.DialogueToDisplay` (`self.DialogueToDisplay`) _output_get)
    (`UserWidget.AddToViewport` _output_get 0)))

(fn `UserConstructionScript`
  (`parent.UserConstructionScript`))