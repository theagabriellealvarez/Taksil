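; BP_MultiClick is an interactable that runs a button-mashing challenge when its static mesh is clicked.
; Activation shows a MultiClick widget and moves input from Tina's controller to this actor.
; Each left click, unless the player is hiding or interacting, adds progress and shakes the camera.
; At 100 progress it restores controller input, removes the widget, resets progress and shows a Fadeout widget.
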(event `self.ReceiveBeginPlay`
  (bind _asbp_tina (cast `/Game/Blueprints/Player/BP_Tina` (`GameplayStatics.GetPlayerPawn` 0)))
  (set `self.As BP Tina` _asbp_tina)
  (bind _asbp_tina_controller (cast `/Game/Blueprints/Player/BP_TinaController` (`GameplayStatics.GetPlayerController` 0)))
  (set `self.As BP Tina Controller` _asbp_tina_controller)
  (bind _asbp_game_mode (cast `/Game/Blueprints/GameMode/BP_GameMode` (`GameplayStatics.GetGameMode`)))
  (set `self.As BP Game Mode` _asbp_game_mode))

(event `Activate Multi Click`
  (bind _returnvalue (`|GenericCreateObject` "/Game/Blueprints/Widgets/BP_MultiClickWidget.BP_MultiClickWidget_C"))
  (set `self.MultiClickWidget` _returnvalue)
  (if (not (`self.isMultiTapEnabled`))
    (`UserWidget.AddToViewport` (`self.MultiClickWidget`) 0)
    (set `self.isMultiTapEnabled` true)
    (`self.DisableInput` (`self.As BP Tina Controller`) null)
    (`self.EnableInput` (`GameplayStatics.GetPlayerController` 0))))

(event `Key|LeftMouseButton`
  (params (Key :type "Key Structure"))
  (:`Pressed`
    (if (`/Game/Blueprints/GameMode/BP_GameMode.isPlayerHiding` (`self.As BP Game Mode`))
      _
      (elif (`/Game/Blueprints/Player/BP_Tina.isInteracting` (`self.As BP Tina`))
        _
        (elif (`self.isMultiTapEnabled`)
          (bind _output_get (set `self.TapProgress` (+ (`self.AddEveryTap`) (`self.TapProgress`))))
          (`KismetSystemLibrary.PrintString` (`KismetStringLibrary.Conv_DoubleToString` _output_get))
          (`GameplayStatics.PlayWorldCameraShake` "/Game/Blueprints/Player/BP_CameraShake.BP_CameraShake_C" (`self.K2_GetActorLocation`) 0.0 10000.0)
          (if (>= (`self.TapProgress`) 100.0)
            (set `self.isMultiTapEnabled` false)
            (`self.DisableInput` (`GameplayStatics.GetPlayerController` 0))
            (`self.EnableInput` (`self.As BP Tina Controller`) null)
            (`Widget.RemoveFromParent` (`self.MultiClickWidget`))
            (set `self.TapProgress` 0.0)
            (bind _returnvalue (`|GenericCreateObject` "/Game/Blueprints/Widgets/temp/Fadeout.Fadeout_C"))
            (`UserWidget.AddToViewport` _returnvalue 0)))))))

(event `self.StaticMesh.OnClicked`
  (params (TouchedComponent :type "PrimitiveComponent Object Reference") (ButtonPressed :type "Key Structure"))
  (`self.Activate Multi Click`))

(fn `Activate MultiClick`)

(fn `UserConstructionScript`)