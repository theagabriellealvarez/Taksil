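; Base interactable actor that the player clicks to pick up and inspect up close.
; A click within range, while the player is neither caught, hiding nor interacting, saves the transform, attaches the actor to the camera manager and moves it into view.
; The player's controller input is disabled while the actor takes input, so dragging with left mouse rotates it.
; Back detaches it, returns it to its saved transform and restores player input.
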(event `self.ReceiveBeginPlay`
  ;[1 1 1] Begin Play (initialize Player Character)
  (bind _asbp_tina (cast `/Game/Blueprints/Player/BP_Tina` (`GameplayStatics.GetPlayerPawn` 0)))
  (set `self.As Player` _asbp_tina)
  (bind _asbp_tina_controller (cast `/Game/Blueprints/Player/BP_TinaController` (`GameplayStatics.GetPlayerController` 0)))
  (set `self.Player Controller` _asbp_tina_controller)
  (bind _asbp_game_mode (cast `/Game/Blueprints/GameMode/BP_GameMode` (`GameplayStatics.GetGameMode`)))
  (set `self.As BP Game Mode` _asbp_game_mode))

(event `CheckDistance`
  ;[1 1 1] Check Distance between player and interactable
  (if (not (`/Game/Blueprints/Player/BP_Tina.isInteracting` (`self.As Player`)))
    (bind _output_get (set `self.isWithinDistance` (< (`KismetMathLibrary.Vector_Distance` (`self.K2_GetActorLocation` self) (`self.K2_GetActorLocation` (`self.As Player`))) 200.0)))
    (if _output_get
      _)))

(event `self.ReceiveActorOnClicked`
  (params (ButtonPressed :type "Key Structure"))
  (bind (_returnvalue_location _returnvalue_rotation) (`KismetMathLibrary.BreakTransform` (`self.GetTransform`)))
  (bind _as_bp_game_mode (`self.As BP Game Mode`))
  (bind _as_player (`self.As Player`))
  ;[1 1 1] If interactable is clicked
  (if (`/Game/Blueprints/GameMode/BP_GameMode.isPlayerCaught` _as_bp_game_mode)
    _
    (elif (not (`/Game/Blueprints/GameMode/BP_GameMode.isPlayerHiding` _as_bp_game_mode))
      (`self.CheckDistance`)
      (if (`self.isWithinDistance`)
        (if (not (`/Game/Blueprints/Player/BP_Tina.isInteracting` (`self.As Player`)))
          (set `self.Original Location` _returnvalue_location)
          (set `self.Original Rotation` _returnvalue_rotation)
          (`self.K2_AttachToComponent` (`PlayerCameraManager.TransformComponent` (`GameplayStatics.GetPlayerCameraManager` 0)) "None" "KeepWorld" "KeepWorld" "KeepWorld")
          (`KismetSystemLibrary.MoveComponentTo` (`self.DefaultSceneRoot`) (200.0 0.0 10.0))
          (set `/Game/Blueprints/Player/BP_Tina.CurrentInteractable` self _as_player)
          (`/Game/Blueprints/Player/BP_Tina.InteractableClicked` _as_player)
          (set `/Game/Blueprints/Player/BP_Tina.isInteracting` true _as_player)
          (`self.DisableInput` (`self.Player Controller`) null)
          (`self.EnableInput` (`GameplayStatics.GetPlayerController` 0)))))))

(event `Back`
  ;[1 1 1] Cancel Inspecting
  (`self.K2_DetachFromActor` "KeepWorld" "KeepWorld" "KeepWorld")
  (`KismetSystemLibrary.MoveComponentTo` (`self.DefaultSceneRoot`) (`self.Original Location`) (`self.Original Rotation`))
  (set `/Game/Blueprints/Player/BP_Tina.isInteracting` false (`self.As Player`))
  (`self.EnableInput` (`self.Player Controller`) null)
  (set `/Game/Blueprints/Player/BP_Tina.CurrentInteractable` null (`self.As Player`)))

(event `Key|LeftMouseButton`
  (params (Key :type "Key Structure"))
  ;[1 1 1] Check if Player is attemtping to rotate interactable
  (:`Pressed`
    (set `self.isRotating` true))
  (:`Released`
    (set `self.isRotating` false)))

(event `InputAxisKey|MouseX`
  (params (AxisValue :type "Float (single-precision)"))
  (bind _defaultsceneroot (`self.DefaultSceneRoot`))
  ;[1 1 1] Rotating logic
  (if (`self.isRotating`)
    (`SceneComponent.K2_SetRelativeRotation` _defaultsceneroot (`KismetMathLibrary.ComposeRotators` (`SceneComponent.RelativeRotation` _defaultsceneroot) (`KismetMathLibrary.MakeRotator` 0.0 0.0 (* AxisValue -5.0))) false false)))

(event `InputAxisKey|MouseY`
  (params (AxisValue :type "Float (single-precision)"))
  (bind _defaultsceneroot (`self.DefaultSceneRoot`))
  ;[1 1 1] Rotating logic
  (if (`self.isRotating`)
    (`SceneComponent.K2_SetRelativeRotation` _defaultsceneroot (`KismetMathLibrary.ComposeRotators` (`SceneComponent.RelativeRotation` _defaultsceneroot) (`KismetMathLibrary.MakeRotator` 0.0 (* AxisValue -5.0))) false false)))

(fn `UserConstructionScript`)