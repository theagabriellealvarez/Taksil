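; Clickable closed door that shows different dialogue depending on whether the player carries a crowbar.
; Hovering outlines it through custom depth and swaps to a grab-hand cursor unless the player is hiding.
; Clicks require the player to be neither caught nor hiding and within range; the crowbar check effectively reads only the last inventory item.
; A dialogue overlay callback activates BP_MultiClick when the crowbar is held.
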(event `self.ReceiveBeginPlay`
  (bind _asbp_game_mode (cast `/Game/Blueprints/GameMode/BP_GameMode` (`GameplayStatics.GetGameMode`)))
  (set `self.As BP Game Mode` _asbp_game_mode)
  (bind _asbp_tina (cast `/Game/Blueprints/Player/BP_Tina` (`GameplayStatics.GetPlayerPawn` 0)))
  (set `self.As BP Tina` _asbp_tina)
  (bind _returnvalue (`|GenericCreateObject` "/Game/Blueprints/DialogueSystem/BP_DialogueOverlay.BP_DialogueOverlay_C"))
  (set `self.DialogueRef` _returnvalue)
  (add `/Game/Blueprints/DialogueSystem/BP_DialogueOverlay.CheckDialogue` (`self.DialogueRef`) (delegate `CheckDialogue`)))

(event `CheckDialogue`
  (if (`self.hasCrowbar`)
    (bind _returnvalue (`GameplayStatics.GetActorOfClass` "/Game/Blueprints/Interactables/BP_MultiClick.BP_MultiClick_C"))
    (`/Game/Blueprints/Interactables/BP_MultiClick.Activate Multi Click` _returnvalue)))

(event `CheckDistance`
  ;[1 1 1] Check Distance between player and searchable
  (if (not (`/Game/Blueprints/Player/BP_Tina.isInteracting` (`self.As BP Tina`)))
    (set `self.Is Within Distance` (< (`KismetMathLibrary.Vector_Distance` (`self.K2_GetActorLocation` self) (`self.K2_GetActorLocation` (`self.As BP Tina`))) 200.0))))

(event `self.StaticMesh.OnBeginCursorOver`
  (params (TouchedComponent :type "PrimitiveComponent Object Reference"))
  ;[1 1 1] Outline object/cursor change
  (if (not (`/Game/Blueprints/GameMode/BP_GameMode.isPlayerHiding` (`self.As BP Game Mode`)))
    (set `PlayerController.CurrentMouseCursor` "GrabHand" (`GameplayStatics.GetPlayerController` 0))
    (`PrimitiveComponent.SetRenderCustomDepth` TouchedComponent true)))

(event `self.StaticMesh.OnEndCursorOver`
  (params (TouchedComponent :type "PrimitiveComponent Object Reference"))
  ;[1 1 1] Outline object/cursor change
  (`PrimitiveComponent.SetRenderCustomDepth` TouchedComponent false)
  (set `PlayerController.CurrentMouseCursor` "Default" (`GameplayStatics.GetPlayerController` 0)))

(event `self.ReceiveActorOnClicked`
  (params (ButtonPressed :type "Key Structure"))
  (bind _as_bp_game_mode (`self.As BP Game Mode`))
  ;[1 1 1] Door logic
  (if (`/Game/Blueprints/GameMode/BP_GameMode.isPlayerCaught` _as_bp_game_mode)
    _
    (elif (not (`/Game/Blueprints/GameMode/BP_GameMode.isPlayerHiding` _as_bp_game_mode))
      (`self.CheckDistance`)
      (if (`self.Is Within Distance`)
        (`self.CheckforCrowbar`)
        (if (`self.hasCrowbar`)
          (`self.DisplayDialogue` (`self.ClosedWCrowDialogue`))
          (else
            (`self.DisplayDialogue` (`self.ClosedNoCrowDialogue`))))))))

(event `self.ReceiveTick`
  (params (DeltaSeconds :type "Float (single-precision)")))

(fn `CheckforCrowbar`
  (bind _inventory (`/Game/Blueprints/Player/BP_Inventory.Inventory` (`/Game/Blueprints/Player/BP_Tina.BP_Inventory` (`self.As BP Tina`))))
  (for (_ _array_index) _inventory
    _)
  (if (`KismetArrayLibrary.Array_IsValidIndex` _inventory)
    (set `self.hasCrowbar` (== (`/Game/Blueprints/ItemDataAssets/BP_ItemDataAssets.Name` (`|GetArrayItem` _inventory _array_index)) "Crowbar"))
    (return)))

(fn `DisplayDialogue`
  (params (Dialogue :type "/Game/Blueprints/DialogueSystem/BP_DialogueDataAsset Object Reference"))
  (bind _dialogueref (`self.DialogueRef`))
  (set `/Game/Blueprints/DialogueSystem/BP_DialogueOverlay.DialogueToDisplay` Dialogue _dialogueref)
  (`UserWidget.AddToViewport` _dialogueref 0))

(fn `UserConstructionScript`)