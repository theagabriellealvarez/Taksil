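; BP_TeddyBear is an interactable teddy bear that yields a Crowbar when the player has scissors.
; The first click on SewHitBox shows dialogue about its back and sets HasInteracted.
; Later clicks add the Crowbar or show no-scissors dialogue, checking only the inventory entry at the finished loop's index, with no guard against repeat rewards.
; DisplayDialogue creates a new BP_DialogueOverlay widget for each message.
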(event `self.SewHitBox.OnClicked`
  (params (TouchedComponent :type "PrimitiveComponent Object Reference") (ButtonPressed :type "Key Structure"))
  (bind _inventory (`/Game/Blueprints/Player/BP_Inventory.Inventory` (`/Game/Blueprints/Player/BP_Tina.BP_Inventory` (`self.As Player`))))
  (for (_ _array_index) _inventory
    _)
  (if (`KismetArrayLibrary.Array_IsValidIndex` _inventory)
    (if (== (`/Game/Blueprints/ItemDataAssets/BP_ItemDataAssets.Name` (`|GetArrayItem` _inventory _array_index)) "Scissors")
      (if (`self.hasInteracted`)
        (`/Game/Blueprints/Player/BP_Inventory.AddItem` (`/Game/Blueprints/Player/BP_Tina.BP_Inventory` (`self.As Player`)) null "/Game/Blueprints/ItemDataAssets/Crowbar.Crowbar")
        (`self.DisplayDialogue` (`self.ScissorsDialogue`))
        (else
          (`self.DisplayDialogue` (`self.TeddyBackDialogue`))
          (set `self.hasInteracted` true)))
      (else
        (if (`self.hasInteracted`) :!label _label
          (`self.DisplayDialogue` (`self.NoScissorsDialogue`))
          (else
            (`self.DisplayDialogue` (`self.TeddyBackDialogue`))
            (set `self.hasInteracted` true)))))
    (else
      (goto _label))))

(fn `DisplayDialogue`
  (params (Dialogue :type "/Game/Blueprints/DialogueSystem/BP_DialogueDataAsset Object Reference"))
  (bind _returnvalue (`|GenericCreateObject` "/Game/Blueprints/DialogueSystem/BP_DialogueOverlay.BP_DialogueOverlay_C"))
  (bind _output_get (set `self.DialogueRef` _returnvalue))
  (set `/Game/Blueprints/DialogueSystem/BP_DialogueOverlay.DialogueToDisplay` Dialogue _output_get)
  (`UserWidget.AddToViewport` _output_get 0))

(fn `UserConstructionScript`
  (`parent.UserConstructionScript`))