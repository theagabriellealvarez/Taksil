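; Interactable swipe quick-time event that challenges Tina with random directions, apparently while hiding, unless she is already caught.
; ActivateQTE disables controller input, creates the prompt widget and binds to the player's end event.
; Tick compares swipes to the prompt, adding time for correct ones and deducting for wrong ones or animation timeouts.
; A Delay-throttled countdown from Tick forces her out of the hiding spot at zero and ends the QTE.
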(event `ActivateQTE`
  ;[1 1 1] Activate QTE
  (bind _asbp_game_mode (cast `/Game/Blueprints/GameMode/BP_GameMode` (`GameplayStatics.GetGameMode`)))
  (if (not (`/Game/Blueprints/GameMode/BP_GameMode.isPlayerCaught` _asbp_game_mode))
    (bind _asbp_tina (cast `/Game/Blueprints/Player/BP_Tina` (`GameplayStatics.GetPlayerPawn` 0)))
    (set `self.Player Ref` _asbp_tina)
    (bind _asbp_tina_controller (cast `/Game/Blueprints/Player/BP_TinaController` (`GameplayStatics.GetPlayerController` 0)))
    (set `self.Player Controller` _asbp_tina_controller)
    (`self.QTE Start`)
    (set `/Game/Blueprints/Player/BP_Tina.SwipeDirection` "None" (`self.Player Ref`))
    (`self.Create QTE Widget`)
    (`self.RandomizeArray`)
    (set `/Game/Blueprints/Widgets/BP_QTE_Widget.QTE Prompt` (`self.QTE Text`) (`self.QTE Widget Ref`))
    (add `/Game/Blueprints/Player/BP_Tina.QteEnd` (`self.Player Ref`) (delegate `call QTE end`))
    (set `self.Seconds` (`self.QTE timer duration`))))

(event `call QTE end`
  ;[1 1 1] Activate QTE
  (`self.QTE End`))

(event `RandomizeArray`
  (bind _randomint (`self.RandomInt`))
  (bind _seconds (`self.Seconds`))
  (bind _qte_widget_ref (`self.QTE Widget Ref`))
  ;[1 1 1] Randomize Direction Array
  (set `self.RandomInt` (`KismetMathLibrary.RandomInteger` 4))
  (set `self.Direction` (`|GetArrayItem` (`self.DirectionArray`) _randomint))
  (set `self.QTE Text` (`|GetArrayItem` (`self.QTE_TextArray`) _randomint))
  (bind _animation (`/Game/Blueprints/Widgets/BP_QTE_Widget.SetDirectionUI` _qte_widget_ref _randomint))
  (`|PlayAnimation` _qte_widget_ref _animation
    (:`Finished`
      (if (== (`/Game/Blueprints/Player/BP_Tina.SwipeDirection` (`self.Player Ref`)) "None")
        (`self.SetNextSwipe`)
        (set `self.Seconds` (`KismetMathLibrary.Clamp` (- _seconds (`self.Deduction(Seconds)`)) 0 _seconds))
        (`/Game/Blueprints/Widgets/BP_QTE_Widget.DeductToTimer` (`self.QTE Widget Ref`))))))

(event `self.ReceiveTick`
  (params (DeltaSeconds :type "Float (single-precision)"))
  (bind _player_ref (`self.Player Ref`))
  (bind _seconds (`self.Seconds`))
  ;[1 1 1] Check Swipe if correct
  (`self.Player Ref`
    (:`then`
      (`self.Timer`)
      (if (== "None" (`self.Direction`))
        (set `/Game/Blueprints/Player/BP_Tina.canSwipe` false _player_ref)
        (else
          (set `/Game/Blueprints/Player/BP_Tina.canSwipe` true _player_ref)
          (if (`/Game/Blueprints/Player/BP_Tina.isQTEActive` _player_ref)
            (if (`/Game/Blueprints/Player/BP_Tina.isSwipeEnd` (`self.Player Ref`))
              (if (== (`self.Direction`) (`/Game/Blueprints/Player/BP_Tina.SwipeDirection` _player_ref))
                (`KismetSystemLibrary.PrintString` "Correct Swipe")
                (`self.SetNextSwipe`)
                (set `self.Seconds` (+ (`self.Addition(Seconds)`) (`self.Seconds`)))
                (`/Game/Blueprints/Widgets/BP_QTE_Widget.AddToTimer` (`self.QTE Widget Ref`))
                (else
                  (`KismetSystemLibrary.PrintString` "Wrong Swipe")
                  (`self.SetNextSwipe`)
                  (set `self.Seconds` (`KismetMathLibrary.Clamp` (- _seconds (`self.Deduction(Seconds)`)) 0 _seconds))
                  (`/Game/Blueprints/Widgets/BP_QTE_Widget.DeductToTimer` (`self.QTE Widget Ref`)))))))))
    (:`else`)))

(event `SetNextSwipe`
  ;[1 1 1] Set Next Direction Swipe
  (set `/Game/Blueprints/Widgets/BP_QTE_Widget.QTE Prompt` "" (`self.QTE Widget Ref`))
  (set `self.Direction` "None")
  (`KismetSystemLibrary.Delay` 1.0)
  (set `/Game/Blueprints/Player/BP_Tina.SwipeDirection` "None" (`self.Player Ref`))
  (`self.RandomizeArray`)
  (set `/Game/Blueprints/Widgets/BP_QTE_Widget.QTE Prompt` (`self.QTE Text`) (`self.QTE Widget Ref`))
  (set `/Game/Blueprints/Player/BP_Tina.isSwipeEnd` false (`self.Player Ref`)))

(event `Create QTE Widget`
  ;[1 1 1] Create QTE Widget
  (bind _returnvalue (`|GenericCreateObject` "/Game/Blueprints/Widgets/BP_QTE_Widget.BP_QTE_Widget_C"))
  (bind _output_get (set `self.QTE Widget Ref` _returnvalue))
  (`UserWidget.AddToViewport` _output_get 0))

(event `QTE Start`
  ;[1 1 1] QTE Start/End
  (`KismetSystemLibrary.Delay` 0.2)
  (set `/Game/Blueprints/Player/BP_Tina.isQTEActive` true (`self.Player Ref`))
  (`self.DisableInput` (`self.Player Controller`) null))

(event `QTE End`
  ;[1 1 1] QTE Start/End
  (set `/Game/Blueprints/Player/BP_Tina.isQTEActive` false (`self.Player Ref`))
  (`Widget.RemoveFromParent` (`self.QTE Widget Ref`))
  (`self.EnableInput` (`self.Player Controller`) null)
  (set `/Game/Blueprints/Player/BP_Tina.SwipeDirection` "None" (`self.Player Ref`)))

(event `Timer`
  (bind _seconds (`self.Seconds`))
  (bind _currenthidable (`/Game/Blueprints/Player/BP_Tina.CurrentHidable` (`self.Player Ref`)))
  ;[1 1 1] Timer
  (`KismetSystemLibrary.Delay` 1.0)
  (if (== (`self.Seconds`) 0)
    (`/Engine/EditorBlueprintResources/StandardMacros.IsValid` (`/Game/Blueprints/Player/BP_Tina.CurrentHidable` (`self.Player Ref`))
      (:`Is Valid`
        (`/Game/Blueprints/HidingSpots/BP_Hideable.Unhide` _currenthidable)
        (`Widget.RemoveFromParent` (`/Game/Blueprints/HidingSpots/BP_Hideable.HideWidget` _currenthidable))
        (`self.QTE End`)
        (set `self.Seconds` (`self.QTE timer duration`))))
    (else
      (set `self.Seconds` (`KismetMathLibrary.Clamp` (- _seconds 1) 0 _seconds)))))

(fn `UserConstructionScript`)