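; BP_Tina is the player Blueprint for Tina, handling touch swipe input during quick-time events and disabling input when GameMode signals the player is caught.
; While a QTE is active, Tick compares touch start to the last stored end point against a distance threshold.
; A DoOnce, reset on release, then reads the current touch and stores the dominant-axis direction as Up, Down, Left or Right.
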(event `self.ReceiveBeginPlay`
  (bind _asbp_tina_controller (cast `/Game/Blueprints/Player/BP_TinaController` (`GameplayStatics.GetPlayerController` 0)))
  (set `self.As Player Controller` _asbp_tina_controller)
  (bind _asbp_game_mode (cast `/Game/Blueprints/GameMode/BP_GameMode` (`GameplayStatics.GetGameMode`)))
  (add `/Game/Blueprints/GameMode/BP_GameMode.PlayerCaught` _asbp_game_mode (delegate `Disable Input`)))

(event `Disable Input`
  (`self.DisableInput` (`self.As Player Controller`) null))

(event `self.ReceiveTick`
  (params (DeltaSeconds :type "Float (single-precision)"))
  (if (`self.isQTEActive`)
    (if (`self.IsPressed`)
      (`self.CheckSwiping`))))

(event `CheckSwiping`
  (if (> (`KismetMathLibrary.VSize2D` (- (`self.TouchStart`) (`self.TouchEnd`))) 300.0)
    (`/Engine/EditorBlueprintResources/StandardMacros.DoOnce` false :!label _label
      (:`Completed`
        (`self.CheckSwipeDirection`)))))

(event `InputTouch`
  (params (Location :type "Vector Structure") (FingerIndex :type "ETouchIndex Enum"))
  (bind _x (.x Location))
  (bind _y (.y Location))
  (:`Pressed`
    (set `self.IsPressed` true)
    (set `self.TouchStart` (`KismetMathLibrary.MakeVector2D` _x _y)))
  (:`Released`
    (set `self.TouchEnd` (`KismetMathLibrary.MakeVector2D` _x _y))
    (goto _label :!via `Reset`)))

(fn `CheckSwipeDirection`
  (bind (_locationx _locationy) (`PlayerController.GetInputTouchState` (`self.As Player Controller`) "Touch1"))
  (bind (_x _y) (`KismetMathLibrary.BreakVector2D` (- (`self.TouchStart`) (`self.TouchEnd`))))
  (set `self.TouchEnd` (`KismetMathLibrary.MakeVector2D` _locationx _locationy))
  (if (> (`KismetMathLibrary.Abs` _x) (`KismetMathLibrary.Abs` _y))
    (if (> _x 0.0)
      (`KismetSystemLibrary.PrintString` "Left")
      (set `self.SwipeDirection` "Left")
      (else
        (`KismetSystemLibrary.PrintString` "Right")
        (set `self.SwipeDirection` "Right")))
    (elif (> _y 0.0)
      (`KismetSystemLibrary.PrintString` "Up")
      (set `self.SwipeDirection` "Up")
      (else
        (`KismetSystemLibrary.PrintString` "Down")
        (set `self.SwipeDirection` "Down")))))

(fn `GetCurrentInteractable`
  (returns (`Current Interactable` :type "/Game/Blueprints/Interactables/BP_Interactable Object Reference"))
  (return (`self.CurrentInteractable`)))

(fn `UserConstructionScript`)