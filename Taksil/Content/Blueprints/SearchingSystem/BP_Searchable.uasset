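; Searchable world object that the player clicks to search, showing dialogue for whether it holds an item.
; Clicks require that the player is neither caught nor hiding and passes a proximity check, which only refreshes while not interacting.
; A search bar widget appears, then after a short delay a DoOnce shows the found or empty dialogue and marks the object searched.
; Hovering an unsearched object shows a grab cursor and custom-depth outline unless hiding.
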(event `self.ReceiveBeginPlay`
  (bind _asbp_game_mode (cast `/Game/Blueprints/GameMode/BP_GameMode` (`GameplayStatics.GetGameMode`)))
  (set `self.As BP Game Mode` _asbp_game_mode)
  (bind _asbp_tina (cast `/Game/Blueprints/Player/BP_Tina` (`GameplayStatics.GetPlayerPawn` 0)))
  (set `self.As Player` _asbp_tina))

(event `CheckDistance`
  ;[1 1 1] Check Distance between player and searchable
  (if (not (`/Game/Blueprints/Player/BP_Tina.isInteracting` (`self.As Player`)))
    (set `self.Is Within Distance` (< (`KismetMathLibrary.Vector_Distance` (`self.K2_GetActorLocation` self) (`self.K2_GetActorLocation` (`self.As Player`))) 200.0))))

(event `self.ReceiveActorOnClicked`
  (params (ButtonPressed :type "Key Structure"))
  (bind _as_bp_game_mode (`self.As BP Game Mode`))
  ;[1 1 1] Search mechanic
  (if (`/Game/Blueprints/GameMode/BP_GameMode.isPlayerCaught` _as_bp_game_mode)
    _
    (elif (not (`/Game/Blueprints/GameMode/BP_GameMode.isPlayerHiding` _as_bp_game_mode))
      (`self.CheckDistance`)
      (if (`self.Is Within Distance`)
        (if (not (`self.hasSearched`))
          (bind _returnvalue (`|CreateWidget` "/Game/Blueprints/SearchingSystem/ProgressBar/BP_SearchBar.BP_SearchBar_C"))
          (bind _output_get (set `self.SearchWidget` _returnvalue))
          (`UserWidget.AddToViewport` _output_get 0)
          (`KismetSystemLibrary.Delay` 1.25)
          (`self.DisplaySearchResult`))))))

(event `DisplaySearchResult`
  ;[1 1 1] Displays if an item has been found or not
  (`/Engine/EditorBlueprintResources/StandardMacros.DoOnce` false
    (:`Completed`
      (bind _returnvalue (`|GenericCreateObject` "/Game/Blueprints/DialogueSystem/BP_DialogueOverlay.BP_DialogueOverlay_C"))
      (bind _output_get (set `self.DialogueRef` _returnvalue))
      (if (`self.hasItem`)
        (set `/Game/Blueprints/DialogueSystem/BP_DialogueOverlay.DialogueToDisplay` (`self.FoundDialogue`) _output_get)
        (else
          (set `/Game/Blueprints/DialogueSystem/BP_DialogueOverlay.DialogueToDisplay` (`self.NoItemDialogue`) _output_get)))
      (`UserWidget.AddToViewport` _output_get 0)
      (set `self.hasSearched` true))))

(event `self.StaticMesh.OnBeginCursorOver`
  (params (TouchedComponent :type "PrimitiveComponent Object Reference"))
  ;[1 1 1] Outline object/cursor change
  (if (`/Game/Blueprints/GameMode/BP_GameMode.isPlayerHiding` (`self.As BP Game Mode`))
    _
    (elif (not (`self.hasSearched`))
      (set `PlayerController.CurrentMouseCursor` "GrabHand" (`GameplayStatics.GetPlayerController` 0))
      (`PrimitiveComponent.SetRenderCustomDepth` TouchedComponent true))))

(event `self.StaticMesh.OnEndCursorOver`
  (params (TouchedComponent :type "PrimitiveComponent Object Reference"))
  ;[1 1 1] Outline object/cursor change
  (`PrimitiveComponent.SetRenderCustomDepth` TouchedComponent false)
  (set `PlayerController.CurrentMouseCursor` "Default" (`GameplayStatics.GetPlayerController` 0)))

(fn `UserConstructionScript`)