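; BP_Ernie is an AI character that wanders between waypoints until told to leave through an exit.
; After spawning its controller and a short delay, it moves to a random waypoint, pauses randomly, then repeats while not exiting.
; AIExit sets IsExiting, stops movement, walks to the given exit actor and destroys itself on arrival.
; Failed moves have no handler, so roaming continues only after a successful move.
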(event `self.ReceiveBeginPlay`
  ;[1 1 1] Begin play
  (`self.SpawnDefaultController`)
  (`KismetSystemLibrary.Delay` 2.0)
  (`self.AI Roam`))

(event `AI Roam`
  (bind _waypoints (`self.Waypoints`))
  (bind _returnvalue (`KismetMathLibrary.RandomInteger` (`KismetArrayLibrary.Array_Length` (`self.Waypoints`))))
  ;[1 1 1] Roaming Logic
  (if (`KismetArrayLibrary.Array_IsValidIndex` _waypoints _returnvalue)
    (`|AIMoveTo` self (0.0 0.0 0.0) (`|GetArrayItem` _waypoints _returnvalue)
      (:`OnSuccess`
        (`KismetSystemLibrary.Delay` (`KismetMathLibrary.RandomFloatInRange` 3.0 5.0))
        (if (not (`self.isExiting`))
          (`self.AI Roam`))))))

(event `AI Exit`
  (params (Exit :type "Actor Object Reference"))
  ;[1 1 1] Exiting Room Logic
  (set `self.isExiting` true)
  (`NavMovementComponent.StopActiveMovement` (`self.CharacterMovement`))
  (`|AIMoveTo` self (0.0 0.0 0.0) Exit
    (:`OnSuccess`
      (`self.K2_DestroyActor`))))

(fn `UserConstructionScript`)