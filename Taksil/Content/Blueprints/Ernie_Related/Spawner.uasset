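; Spawner actor that creates and retires the BP_Ernie AI character.
; SpawnErnie spawns Ernie at the spawner's transform, stores the reference and hands over the spawner's Waypoints.
; DespawnErnie calls Ernie's AIExit with itself as argument, then binds to Ernie's OnDestroyed to broadcast OnExit once Ernie is destroyed.
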(event `Spawn Ernie`
  (bind _returnvalue (`|SpawnActorFromClass` "/Game/Blueprints/Ernie_Related/BP_Ernie.BP_Ernie_C" (`self.GetTransform` self) "Undefined" "MultiplyWithRoot" null null))
  (set `self.Ernie` _returnvalue)
  (set `/Game/Blueprints/Ernie_Related/BP_Ernie.Waypoints` (`self.Waypoints`) _returnvalue))

(event `Despawn Ernie`
  (`/Game/Blueprints/Ernie_Related/BP_Ernie.AI Exit` (`self.Ernie`) self)
  (add `self.OnDestroyed` (`self.Ernie`) (delegate `OnDestroyed_Event`)))

(event `OnDestroyed_Event` :!signature `self.OnDestroyed`
  (params (DestroyedActor :type "Actor Object Reference"))
  (`self.OnExit`))

(fn `UserConstructionScript`)