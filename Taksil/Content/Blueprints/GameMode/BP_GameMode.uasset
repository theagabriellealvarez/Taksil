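; Game mode that runs a timed Ernie visit cycle and shows the interactable UI in a top-down game.
; On BeginPlay it creates the UI widget, binds to the player character's click event to add it to the viewport, and finds the level's Spawner.
; Ernie spawns and despawns through the Spawner after random delays, and the Spawner's OnExit event restarts the cycle.
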(event `self.ReceiveBeginPlay`
  (bind _returnvalue (`|CreateWidget` "/Game/Blueprints/Widgets/BP_InteractableUI.BP_InteractableUI_C"))
  (set `self.InteractableWidget` _returnvalue)
  (bind _asbp_top_down_character (cast `/Game/Blueprints/Player/BP_TopDownCharacter` (`GameplayStatics.GetPlayerPawn` 0)))
  (add `/Game/Blueprints/Player/BP_TopDownCharacter.InteractableClicked` _asbp_top_down_character (delegate `InteractableClicked`))
  (bind _returnvalue_2 (`GameplayStatics.GetActorOfClass` "/Game/Blueprints/Ernie_Related/Spawner.Spawner_C"))
  (set `self.Spawner` _returnvalue_2)
  (`self.Spawn Ernie`)
  (add `/Game/Blueprints/Ernie_Related/Spawner.OnExit` _returnvalue_2 (delegate `On Exit`)))

(event `On Exit`
  (`self.Spawn Ernie`))

(event `InteractableClicked`
  (`UserWidget.AddToViewport` (`self.InteractableWidget`) 0))

(event `Spawn Ernie`
  (`KismetSystemLibrary.Delay` (`KismetMathLibrary.RandomFloatInRange` 10.0 20.0))
  (`/Game/Blueprints/Ernie_Related/Spawner.Spawn Ernie` (`self.Spawner`))
  (`KismetSystemLibrary.Delay` (`KismetMathLibrary.RandomFloatInRange` 20.0 25.0))
  (`/Game/Blueprints/Ernie_Related/Spawner.Despawn Ernie` (`self.Spawner`)))

(fn `UserConstructionScript`)